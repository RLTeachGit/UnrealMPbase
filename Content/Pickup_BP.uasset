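; Pickup actor that takes on its instigator's chest colour and damages any ThirdPersonCharacter that overlaps it.
; The construction script creates a dynamic material instance, which SetColour tints on BeginPlay.
; Overlaps are handled only on the server, where HitPickup lowers Health by one using a set so its OnNotify fires.
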(event Custom|HitPickup
  (params (Player :type Third%20Person%20Character%20Object%20Reference))
  ;[1 1 1] The needs to be a set for the OnNotify to fire
  (Variables|/Game/ThirdPersonBP/Blueprints/ThirdPersonCharacter.ThirdPersonCharacter_C|SetHealth Player (- (Variables|/Game/ThirdPersonBP/Blueprints/ThirdPersonCharacter.ThirdPersonCharacter_C|GetHealth Player) 1)))

(event EventBeginPlay
  (bind _asthird_person_character (Utilities|Casting|CastToThirdPersonCharacter (Game|GetInstigator)))
  (CallFunction|SetColour (Variables|/Game/ThirdPersonBP/Blueprints/ThirdPersonCharacter.ThirdPersonCharacter_C|GetChestColour _asthird_person_character)))

(event Collision|EventActorBeginOverlap
  (params (OtherActor :type Actor%20Object%20Reference))
  (if (Networking|IsServer)
    (bind _asthird_person_character (Utilities|Casting|CastToThirdPersonCharacter OtherActor))
    (CallFunction|HitPickup _asthird_person_character)))

(event EventTick
  (params (DeltaSeconds :type Float%20%28single-precision%29)))

(fn ConstructionScript
  (bind _returnvalue (Rendering|Material|CreateDynamicMaterialInstance (Variables|Debug|GetStaticMeshComponent) 0 "/Game/BasicColour.BasicColour" "None" :!class /Script/Engine.PrimitiveComponent))
  (Variables|Default|SetPickupMaterial _returnvalue))

(fn SetColour
  (params (Colour :type Linear%20Color%20Structure))
  (Rendering|Material|SetVectorParameterValue (Variables|Default|GetPickupMaterial) (Variables|Default|GetColourName) Colour :!class /Script/Engine.MaterialInstanceDynamic))